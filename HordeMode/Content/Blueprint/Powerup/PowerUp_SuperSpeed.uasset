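; Super-speed power-up Blueprint that temporarily doubles the movement speed of the actor that activates it.
; On activation it stores that actor and sets its CharacterMovementComponent's MaxWalkSpeed to twice GetMaxSpeed, which reflects the current movement mode.
; On expiry it sets MaxWalkSpeed to half the then-current GetMaxSpeed, calling the parent's expiry logic only if the stored actor is still valid.
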(event EventOnActivated
  (params (ForActor :type Actor%20Object%20Reference))
  (bind _returnvalue (Actor|GetComponentbyClass ForActor "/Script/Engine.CharacterMovementComponent"))
  (Variables|Default|SetPlayerThatActivated ForActor)
  (Variables|/Script/Engine.CharacterMovementComponent|SetMaxWalkSpeed _returnvalue (* (Class|MovementComponent|GetMaxSpeed _returnvalue) 2.0)))

(event EventOnExpired
  (bind _playerthatactivated (Variables|Default|GetPlayerThatActivated))
  (bind _returnvalue (Actor|GetComponentbyClass _playerthatactivated "/Script/Engine.CharacterMovementComponent"))
  (Utilities|IsValid _playerthatactivated
    (:Is%20Valid
      (Variables|/Script/Engine.CharacterMovementComponent|SetMaxWalkSpeed _returnvalue (/ (Class|MovementComponent|GetMaxSpeed _returnvalue) 2.0))
      (|CallParentFunction))))

(fn ConstructionScript)