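; Player character Blueprint that manages the gameplay HUD widgets.
; On BeginPlay, the locally controlled player gets crosshair, health and ammo count widgets, which are removed along with the play-area warning when health reaches zero.
; PickupComp's best-interactable event shows or hides a reusable pickup prompt for the local player.
; Leaving and entering play-area events update that state and add or remove the warning widget.
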(event OnHealthChanged(HealthComp)
  (params (HealthComponent :type S%20Health%20Component%20Object%20Reference) (Health :type Float%20%28single-precision%29) (HealthDelta :type Float%20%28single-precision%29) (DamageType :type Damage%20Type%20Object%20Reference) (InstigatedBy :type Controller%20Object%20Reference) (DamageCauser :type Actor%20Object%20Reference))
  ;[1 1 1] Removes gameplay widget on death
  (if (== Health 0.0)
    (Widget|RemovefromParent (Variables|Default|GetAmmoCountWidget))
    (Widget|RemovefromParent (Variables|Default|GetHealthWidget))
    (Widget|RemovefromParent (Variables|Default|GetCrosshairWidget))
    (Widget|RemovefromParent (Variables|Default|GetPlayAreaWidget))))

(event ActiveBestInteractable(PickupComp)
  (bind _pickupcomp (Variables|Default|GetPickupComp))
  (if (Pawn|IsLocallyControlled)
    ;[1 1 1] Pick up system Widget
    (Utilities|IsValid _pickupcomp
      (:Is%20Valid
        (Utilities|IsValid (Variables|/Script/HordeMode.PickUpComponent|GetInteractableItem _pickupcomp)
          (:Is%20Valid
            (Utilities|IsValid (Variables|Default|GetPickupWidget)
              (:Is%20Valid
                (UserInterface|Viewport|AddtoViewport (Variables|Default|GetPickupWidget) 0))
              (:Is%20Not%20Valid
                (CallFunction|CreatePickupWidget))))
          (:Is%20Not%20Valid
            (Utilities|IsValid (Variables|Default|GetPickupWidget)
              (:Is%20Valid
                (CallFunction|RemovePickupwidget)))))))))

(event Custom|LeavingPlayArea
  ;[1 1 1] Creates or removes Warning widget base on if the player is in the play area.
  (if (not (Variables|Default|GetbIsDead))
    (Class|SCharacter|SetPlayArea false)
    (bind _returnvalue (UserInterface|CreateWidget "/Game/Blueprint/UI/WBP_PlayZone.WBP_PlayZone_C"))
    (Variables|Default|SetPlayAreaWidget _returnvalue)
    (UserInterface|Viewport|AddtoViewport _returnvalue 0)))

(event Custom|EnteringPlayArea
  (bind _playareawidget (Variables|Default|GetPlayAreaWidget))
  ;[1 1 1] Creates or removes Warning widget base on if the player is in the play area.
  (Class|SCharacter|SetPlayArea true)
  (Utilities|IsValid _playareawidget
    (:Is%20Valid
      (Widget|RemovefromParent _playareawidget))))

(event Custom|CreatePickupWidget
  ;[1 1 1] Pick up system Widget
  (bind _asplayer_controller (Utilities|Casting|CastToPlayerController (Pawn|GetController)))
  (bind _returnvalue (UserInterface|CreateWidget "/Game/Blueprint/UI/WBP_Interactable.WBP_Interactable_C" _asplayer_controller))
  (bind _output_get (Variables|Default|SetPickupWidget _returnvalue))
  (UserInterface|Viewport|AddtoViewport _output_get 0))

(event Custom|RemovePickupwidget
  (bind _pickupwidget (Variables|Default|GetPickupWidget))
  ;[1 1 1] Pick up system Widget
  (Utilities|IsValid _pickupwidget
    (:Is%20Valid
      (Widget|RemovefromParent _pickupwidget))))

(event EventBeginPlay
  (if (Pawn|IsLocallyControlled)
    (Utilities|FlowControl|Sequence
      (:then_0
        ;[1 1 1] Creates the gameplay widget when the create is created
        (bind _returnvalue (UserInterface|CreateWidget "/Game/Blueprint/UI/WBP_CrossHair.WBP_CrossHair_C"))
        (Variables|Default|SetCrosshairWidget _returnvalue)
        (UserInterface|Viewport|AddtoViewport _returnvalue 0))
      (:then_1
        (bind _returnvalue_2 (UserInterface|CreateWidget "/Game/Blueprint/UI/WBP_HealthIndicator.WBP_HealthIndicator_C"))
        (Variables|Default|SetHealthWidget _returnvalue_2)
        (UserInterface|Viewport|AddtoViewport _returnvalue_2 0))
      (:then_2
        (bind _asplayer_controller (Utilities|Casting|CastToPlayerController (Pawn|GetController)))
        (bind _returnvalue_3 (UserInterface|CreateWidget "/Game/Blueprint/UI/WBP_AmmoCount.WBP_AmmoCount_C" _asplayer_controller))
        (Variables|Default|SetAmmoCountWidget _returnvalue_3)
        (UserInterface|Viewport|AddtoViewport _returnvalue_3 0)))))

(fn ConstructionScript)