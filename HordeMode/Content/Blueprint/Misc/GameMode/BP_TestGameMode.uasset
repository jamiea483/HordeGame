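; BP_TestGameMode is a test game mode that spawns AI enemies and handles kill scoring.
; SpawnNewBot runs an EQS query for spawn locations, then spawns BP_AdavanceAI or TrackerBot at random at each result, with debug spheres.
; When a non-player pawn dies, the kill event updates the game state's enemies-left count and adds score and a kill to the supplied PlayerController's SPlayerState, printing the score.
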(event Custom|OnQueryFinishedEvent_Event_0
  (params (QueryInstance :type Env%20Query%20Instance%20Blueprint%20Wrapper%20Object%20Reference) (QueryStatus :type EEnvQueryStatus%20Enum :default "Processing"))
  (switch Utilities|FlowControl|Switch|SwitchonEEnvQueryStatus QueryStatus
    (:Success
      (bind _resultlocations (AI|EQS|GetQueryResultsasLocations QueryInstance))
      (for _array_element _resultlocations
        (Rendering|Debug|DrawDebugSphere _array_element 5e+01 12 "(R=1.000000,G=0.097827,B=0.000000,A=1.000000)" 2.0 1.0)
        (Game|SpawnActorfromClass (select (<= (Math|Random|RandomIntegerinRange 0 100) 40) "/Game/Blueprint/AI/Advance/BP_AdavanceAI.BP_AdavanceAI_C" "/Game/Blueprint/AI/Basic/TrackerBot.TrackerBot_C") (Math|Transform|MakeTransform _array_element) "AdjustIfPossibleButDontSpawnIfColliding" 0 0)))))

(event Custom|OnActorKilledEvent
  (params (VictimActor :type Actor%20Object%20Reference) (KillerActor :type Actor%20Object%20Reference) (PlayerController :type Controller%20Object%20Reference))
  (bind _aspawn (Utilities|Casting|CastToPawn VictimActor))
  (if (not (Pawn|IsPlayerControlled _aspawn))
    (CallFunction|EnemyleftUI)
    (bind _assplayer_state (Utilities|Casting|CastToSPlayerState (Variables|/Script/Engine.Pawn|GetPlayerState (Pawn|GetControlledPawn PlayerController))))
    (Class|SPlayerState|AddScore _assplayer_state 1e+01)
    (Class|SPlayerState|AddKill _assplayer_state 1.0)
    (Development|PrintString (Utilities|String|ToString(Float) (Variables|/Script/Engine.PlayerState|GetScore _assplayer_state)) true true "(R=1.000000,G=0.093222,B=0.083274,A=1.000000)" 1.0)))

(event Custom|EnemyleftUI
  (bind _asbp_sgame_state (Utilities|Casting|CastToBP_SGameState (Game|GetGameState)))
  (Class|SGameState|SetEnemysLeft _asbp_sgame_state -1))

(event EventBeginPlay
  (EventDispatchers|BindEventtoOnActorKilled (delegate Custom|OnActorKilledEvent)))

(event EventSpawnNewBot
  (bind _returnvalue (AI|EQS|RunEQSQuery "/Game/Blueprint/Misc/EQS_FindSpawnLocation.EQS_FindSpawnLocation" self "RandomBest25Pct"))
  (EventDispatchers|AssignOnQueryFinishedEvent _returnvalue (delegate Custom|OnQueryFinishedEvent_Event_0)))

(fn ConstructionScript)