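; Grenade actor that explodes on a short fixed timer after it spawns.
; BeginPlay starts the timer by function name, and Explode applies radial damage at the actor's location, crediting the grenade and its instigator controller.
; A Radius variable sizes both the damage area and a briefly drawn debug sphere, the only visual in the graph, before the actor destroys itself.
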(event Custom|Explode
  (bind _self self)
  (bind _returnvalue (Transformation|GetActorLocation _self))
  (Game|Damage|ApplyRadialDamage 4e+01 _returnvalue (Variables|Default|GetRadius) 0 0 self (Game|GetInstigatorController) false "ECC_Visibility")
  (Rendering|Debug|DrawDebugSphere _returnvalue (Variables|Default|GetRadius) 12 "(R=0.897111,G=0.449886,B=1.000000,A=1.000000)" 1.0 1.0)
  (Actor|DestroyActor))

(event EventBeginPlay
  (Utilities|Time|SetTimerbyFunctionName 0 "Explode" 1.0))

(fn ConstructionScript)